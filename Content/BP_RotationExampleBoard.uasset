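; Example board that shows draggable trigger percentages driving a head's yaw, a lamp and a poseable mesh's head bone scale.
; On BeginPlay it takes the bulb from a child actor, turns off its physics, attaches it to the board and sets its light color.
; Comp_ListenToTrigger's constant trigger event routes each percent by name, lerping rotation or scale directly and forwarding the center value to the bulb's own listener.
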(event `self.ReceiveBeginPlay`
  (bind _asbp_lights_bulb (cast `/Game/AVRFramework/Experiences/Demospace/Examples/Snapping/BP_Lights_Bulb` (`ChildActorComponent.ChildActor` (`self.LampExampleChild`))))
  (bind _output_get (set `self.LightBulb` _asbp_lights_bulb))
  (`PrimitiveComponent.SetSimulatePhysics` (`/Game/AVRFramework/Experiences/Demospace/Examples/Snapping/BP_Lights_Bulb.StaticMesh` _output_get) false)
  (`self.K2_AttachToActor` _output_get self "None" "KeepWorld" "KeepWorld" "KeepWorld" false)
  (`/Game/AVRFramework/Blueprints/Components/State/Comp_Light.SetNewLightColor` (`/Game/AVRFramework/Experiences/Demospace/Examples/Snapping/BP_Lights_Bulb.Comp_Light` (`self.LightBulb`)) "NewEnumerator12"))

(event `self.ReceiveTick`
  (params (DeltaSeconds :type "Float (single-precision)")))

(event `self.Comp_ListenToTrigger.TriggerConstant`
  (params (Name :type Name) (Distance :type "Float (single-precision)") (Percent :type "Float (single-precision)") (Set :type "/Game/AVRFramework/Structs/Struct_Section Structure") (Velocity :type "Float (single-precision)") (Source :type "Actor Object Reference") (Pawn :type "/Game/AVRFramework/Blueprints/Pawn/BP_Pawn_Base Object Reference"))
  (switch `name` Name
    (:`DragLowerLeft`
      (`SceneComponent.K2_SetRelativeRotation` (`self.HeadExample`) (`KismetMathLibrary.MakeRotator` 0.0 0.0 (`KismetMathLibrary.Lerp` -90.0 90.0 Percent)) false false))
    (:`DragCenter`
      ;[1 1 1] Lamp
      (bind _lightbulb (`self.LightBulb`)
        (:`then`
          (`/Game/AVRFramework/Blueprints/Components/State/Comp_ListenToTrigger.ConstantTriggers` :`self` (`/Game/AVRFramework/Experiences/Demospace/Examples/Snapping/BP_Lights_Bulb.Comp_ListenToTrigger` _lightbulb) :`Procent` Percent :`Source` self))
        (:`else`)))
    (:`DragLowerRight`
      ;[1 1 1] Head
      (`PoseableMeshComponent.SetBoneScaleByName` (`self.PoseableMesh`) "head" (`KismetMathLibrary.Conv_DoubleToVector` (`KismetMathLibrary.Lerp` 0.2 1.0 Percent)) "WorldSpace"))))

(fn `UserConstructionScript`)