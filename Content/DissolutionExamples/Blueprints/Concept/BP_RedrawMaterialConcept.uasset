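; BP_RedrawMaterialConcept is a concept actor that redraws materials from source actors onto paired target actors in the SourceTargetActors map.
; Activate draws each source mesh's first material into a new 512x512 render target, feeds it as a texture to a dynamic instance of M_RedrawConceptMaterial, and assigns that to the target mesh.
; Deactivate sets slot 0 on each target's static mesh component to an empty material, removing the override.
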(event `self.ReceiveBeginPlay`)

(event `/Game/DissolutionExamples/Blueprints/Interface/BP_ActivationInterface.Activate`
  (params (Appearance :type Boolean))
  (bind _sourcetargetactors (`self.SourceTargetActors`))
  (bind _keys (`BlueprintMapLibrary.Map_Keys` _sourcetargetactors))
  (for _array_element _keys
    (`/Engine/EditorBlueprintResources/StandardMacros.IsValid` _array_element
      (:`Is Valid`
        (bind _returnvalue (`self.GetComponentByClass` _array_element "/Script/Engine.MeshComponent"))
        (`/Engine/EditorBlueprintResources/StandardMacros.IsValid` _returnvalue
          (:`Is Valid`
            (bind _value (`BlueprintMapLibrary.Map_Find` _sourcetargetactors _array_element))
            (`/Engine/EditorBlueprintResources/StandardMacros.IsValid` _value
              (:`Is Valid`
                (bind _returnvalue_2 (`self.GetComponentByClass` _value "/Script/Engine.MeshComponent"))
                (`/Engine/EditorBlueprintResources/StandardMacros.IsValid` _returnvalue_2
                  (:`Is Valid`
                    (bind _returnvalue_3 (`KismetRenderingLibrary.CreateRenderTarget2D` 512 512 "RTF_RGBA16f" (struct)))
                    (`KismetRenderingLibrary.DrawMaterialToRenderTarget` _returnvalue_3 (`PrimitiveComponent.GetMaterial` _returnvalue 0))
                    (bind _returnvalue_4 (`KismetMaterialLibrary.CreateDynamicMaterialInstance` "/Game/DissolutionExamples/Materials/M_RedrawConceptMaterial.M_RedrawConceptMaterial"))
                    (`MaterialInstanceDynamic.SetTextureParameterValue` _returnvalue_4 "Texture" _returnvalue_3)
                    (`PrimitiveComponent.SetMaterial` _returnvalue_2 0 _returnvalue_4)))))))))))

(event `/Game/DissolutionExamples/Blueprints/Interface/BP_ActivationInterface.Deactivate`
  (bind _values (`BlueprintMapLibrary.Map_Values` (`self.SourceTargetActors`)))
  (for _array_element _values
    (`/Engine/EditorBlueprintResources/StandardMacros.IsValid` _array_element
      (:`Is Valid`
        (bind _returnvalue (`self.GetComponentByClass` _array_element "/Script/Engine.StaticMeshComponent"))
        (`/Engine/EditorBlueprintResources/StandardMacros.IsValid` _returnvalue
          (:`Is Valid`
            (`PrimitiveComponent.SetMaterial` _returnvalue 0 null)))))))

(fn `UserConstructionScript`)