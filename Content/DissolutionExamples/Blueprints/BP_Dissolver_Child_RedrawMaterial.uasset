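; Dissolver child Blueprint that dissolves an actor into Niagara effects textured with its own redrawn materials.
; Dissolve gathers the actor's static and skeletal mesh components, drawing each one's first material into a new render target.
; That texture feeds a dynamic sprite material, passed with mesh, center and lifetime to an auto-destroying Niagara component per mesh.
; It returns those components; Activate, Deactivate and construction defer to the parent.
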(event `self.ReceiveBeginPlay`)

(event `/Game/DissolutionExamples/Blueprints/Interface/BP_ActivationInterface.Activate`
  (params (Appearance :type Boolean))
  (`parent.Activate` Appearance))

(event `/Game/DissolutionExamples/Blueprints/Interface/BP_ActivationInterface.Deactivate`
  (`parent.Deactivate`))

(fn `Dissolve`
  (params (Actor :type "Actor Object Reference") (InAsset :type "NiagaraSystem Object Reference"))
  (returns (NiagaraComponents :type "Array of NiagaraComponent Object Reference"))
  (locals (LocalNiagaraComponents :type "Array of NiagaraComponent Object Reference") (LocalComponents :type "Array of PrimitiveComponent Object Reference") (LocalSpriteMaterial :type "MaterialInstanceDynamic Object Reference"))
  (bind _localcomponents (`local.LocalComponents`))
  (bind _returnvalue (`self.K2_GetComponentsByClass` (`local.Actor`) "/Script/Engine.SkeletalMeshComponent"))
  (bind _returnvalue_2 (`self.K2_GetComponentsByClass` (`local.Actor`) "/Script/Engine.StaticMeshComponent"))
  (`/Engine/EditorBlueprintResources/StandardMacros.IsValid` Actor
    (:`Is Valid`
      (`/Engine/EditorBlueprintResources/StandardMacros.IsValid` InAsset
        (:`Is Valid`
          (`|ExecutionSequence`
            (:`then_0`
              (if (> (`KismetArrayLibrary.Array_Length` _returnvalue_2) 0)
                (`KismetArrayLibrary.Array_Append` _localcomponents _returnvalue_2)))
            (:`then_1`
              (if (> (`KismetArrayLibrary.Array_Length` _returnvalue) 0)
                (`KismetArrayLibrary.Array_Append` _localcomponents _returnvalue)))
            (:`then_2`
              (for _array_element (`local.LocalComponents`)
                (`|ExecutionSequence`
                  (:`then_0`
                    (bind _returnvalue_3 (`KismetRenderingLibrary.CreateRenderTarget2D` 512 512 "RTF_RGBA16f" (struct)))
                    (`KismetRenderingLibrary.DrawMaterialToRenderTarget` _returnvalue_3 (`PrimitiveComponent.GetMaterial` _array_element 0))
                    (bind _returnvalue_4 (`KismetMaterialLibrary.CreateDynamicMaterialInstance` "/Game/DissolutionExamples/Materials/M_SpriteRedrawMaterial.M_SpriteRedrawMaterial"))
                    (`MaterialInstanceDynamic.SetTextureParameterValue` _returnvalue_4 "RedrawMaterialTexture" _returnvalue_3)
                    (set `local.LocalSpriteMaterial` _returnvalue_4))
                  (:`then_1`
                    (bind _returnvalue_5 (`AddComponent|NODE_AddNiagaraComponent-0` :`bManualAttachment` true :`RelativeTransform` (`KismetMathLibrary.Conv_VectorToTransform` (`self.K2_GetActorLocation` (`local.Actor`)))))
                    (`KismetArrayLibrary.Array_Add` (`local.LocalNiagaraComponents`) _returnvalue_5)
                    (`NiagaraComponent.SetAsset` _returnvalue_5 (`local.InAsset`))
                    (`NiagaraComponent.SetVariableMaterial` _returnvalue_5 "Material" (`local.LocalSpriteMaterial`))
                    (`NiagaraComponent.SetVariableVec3` _returnvalue_5 "Center" (`self.K2_GetActorLocation`))
                    (`NiagaraComponent.SetNiagaraVariableFloat` _returnvalue_5 "Lifetime" (`self.Lifetime`))
                    (`NiagaraComponent.SetAutoDestroy` _returnvalue_5 true))
                  (:`then_2`
                    (bind _asstatic_mesh_component (cast `StaticMeshComponent` _array_element))
                    (`NiagaraFunctionLibrary.OverrideSystemUserVariableStaticMeshComponent` _returnvalue_5 "StaticMesh" _asstatic_mesh_component))
                  (:`then_3`
                    (bind _asskeletal_mesh_component (cast `SkeletalMeshComponent` _array_element))
                    (`NiagaraFunctionLibrary.OverrideSystemUserVariableSkeletalMeshComponent` _returnvalue_5 "SkeletalMesh" _asskeletal_mesh_component))
                  (:`then_4`
                    (`NiagaraComponent.ReinitializeSystem` _returnvalue_5)))))
            (:`then_3`
              (return (`local.LocalNiagaraComponents`)))))
        (:`Is Not Valid`
          (return (`local.LocalNiagaraComponents`)))))
    (:`Is Not Valid`
      (return (`local.LocalNiagaraComponents`)))))

(fn `UserConstructionScript`
  (`parent.UserConstructionScript`))