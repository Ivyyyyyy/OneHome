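; Dissolver child that drives a Niagara dissolve or appearance effect on target actors by sweeping a capture rig along a spline.
; Activation creates orthographic-width scene captures into base color, normal and depth render targets, showing only mapped actors.
; A timeline moves the rig and updates material parameter collection position and direction, reversed for appearance.
; Dissolve feeds those textures to one Niagara component per system asset; deactivation clears targets and destroys captures.
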(event `self.ReceiveBeginPlay`
  (`SceneComponent.SetVisibility` (`self.Decal`) (`self.DissolveAreaVisibility`) false))

(event `/Game/DissolutionExamples/Blueprints/Interface/BP_ActivationInterface.Activate`
  (params (Appearance :type Boolean))
  (bind _trackspline (`self.TrackSpline`))
  (bind _scene (`self.Scene`))
  (bind _returnvalue (* (`self.Width`) 0.5))
  (bind _returnvalue_2 (* (`self.Width`) 2))
  (`|ExecutionSequence`
    (:`then_0`
      (`|ExecutionSequence`
        (:`then_0`
          (bind _returnvalue_3 (`KismetRenderingLibrary.CreateRenderTarget2D` _returnvalue_2 _returnvalue_2))
          (bind _output_get (set `self.BaseColorTexture` _returnvalue_3))
          (bind _returnvalue_4 (`AddComponent|NODE_AddSceneCaptureComponent2D-0`))
          (set `SceneCaptureComponent2D.TextureTarget` _output_get _returnvalue_4)
          (set `SceneCaptureComponent2D.OrthoWidth` (`KismetMathLibrary.Conv_IntToDouble` (`self.Width`)) _returnvalue_4)
          (`SceneComponent.K2_AttachToComponent` _returnvalue_4 (`self.Scene`) "None" "KeepWorld" "KeepWorld" "KeepWorld" true)
          (`KismetArrayLibrary.Array_AddUnique` (`self.SceneCaptureComponents`) _returnvalue_4))
        (:`then_1`
          (bind _returnvalue_5 (`KismetRenderingLibrary.CreateRenderTarget2D` _returnvalue_2 _returnvalue_2))
          (bind _output_get_2 (set `self.NormalTexture` _returnvalue_5))
          (bind _returnvalue_6 (`AddComponent|NODE_AddSceneCaptureComponent2D-1`))
          (set `SceneCaptureComponent2D.TextureTarget` _output_get_2 _returnvalue_6)
          (set `SceneCaptureComponent2D.OrthoWidth` (`KismetMathLibrary.Conv_IntToDouble` (`self.Width`)) _returnvalue_6)
          (`SceneComponent.K2_AttachToComponent` _returnvalue_6 (`self.Scene`) "None" "KeepWorld" "KeepWorld" "KeepWorld" true)
          (`KismetArrayLibrary.Array_AddUnique` (`self.SceneCaptureComponents`) _returnvalue_6))
        (:`then_2`
          (bind _returnvalue_7 (`KismetRenderingLibrary.CreateRenderTarget2D` _returnvalue_2 _returnvalue_2))
          (bind _output_get_3 (set `self.DepthTexture` _returnvalue_7))
          (bind _returnvalue_8 (`AddComponent|NODE_AddSceneCaptureComponent2D-2`))
          (set `SceneCaptureComponent2D.TextureTarget` _output_get_3 _returnvalue_8)
          (set `SceneCaptureComponent2D.OrthoWidth` (`KismetMathLibrary.Conv_IntToDouble` (`self.Width`)) _returnvalue_8)
          (`SceneComponent.K2_AttachToComponent` _returnvalue_8 (`self.Scene`) "None" "KeepWorld" "KeepWorld" "KeepWorld" true)
          (`KismetArrayLibrary.Array_AddUnique` (`self.SceneCaptureComponents`) _returnvalue_8))
        (:`then_3`
          (bind _keys (`BlueprintMapLibrary.Map_Keys` (`self.ActorNiagaraSystemMap`)))
          (for _array_element _keys
            (`|ExecutionSequence`
              (:`then_0`
                (for _array_element_2 (`self.SceneCaptureComponents`)
                  (`SceneCaptureComponent.ShowOnlyActorComponents` _array_element_2 _array_element false))))))))
    (:`then_1`
      (`parent.Activate` Appearance)
      (bind (_direction _newtrack_0) (`Timeline|Timeline_0` :!via `PlayFromStart` :!label _label)
        (:`Update`
          (`|ExecutionSequence`
            (:`then_0`
              (bind _returnvalue_9 (* (`SplineComponent.GetSplineLength` _trackspline) _newtrack_0))
              (bind _returnvalue_10 (`SplineComponent.GetLocationAtDistanceAlongSpline` _trackspline _returnvalue_9 "World"))
              (`SceneComponent.K2_SetWorldLocation` _scene _returnvalue_10 false false)
              (bind _returnvalue_11 (`SplineComponent.GetDirectionAtDistanceAlongSpline` _trackspline _returnvalue_9 "World"))
              (bind _returnvalue_12 (select `bool` Appearance :`false` _returnvalue_11 :`true` (* _returnvalue_11 -1.0)))
              (bind _returnvalue_13 (`KismetMathLibrary.MakeRotFromX` _returnvalue_12))
              (`SceneComponent.K2_SetWorldRotation` _scene _returnvalue_13 false false)
              (if (`self.DissolveAreaVisibility`)
                (`KismetSystemLibrary.DrawDebugBox` _returnvalue_10 (`KismetMathLibrary.MakeVector` 0.0 _returnvalue _returnvalue) (struct :`R` 1.0 :`A` 1.0) _returnvalue_13 0.0 2.0)))
            (:`then_1`
              (`KismetMaterialLibrary.SetVectorParameterValue` "/Game/DissolutionExamples/Materials/MPC_DissolutionMaterialParameterCollection.MPC_DissolutionMaterialParameterCollection" "DissolutionAttractor" (`KismetMathLibrary.Conv_VectorToLinearColor` _returnvalue_10)))
            (:`then_2`
              (`KismetMaterialLibrary.SetVectorParameterValue` "/Game/DissolutionExamples/Materials/MPC_DissolutionMaterialParameterCollection.MPC_DissolutionMaterialParameterCollection" "ForwardVector" (`KismetMathLibrary.Conv_VectorToLinearColor` _returnvalue_12)))))))))

(event `/Game/DissolutionExamples/Blueprints/Interface/BP_ActivationInterface.Deactivate`
  (bind _trackspline (`self.TrackSpline`))
  (bind _scenecapturecomponents (`self.SceneCaptureComponents`))
  (`parent.Deactivate`)
  (`|ExecutionSequence`
    (:`then_0`
      (goto _label :!via `Stop`))
    (:`then_1`
      (`|ExecutionSequence`
        (:`then_0`
          (`SceneComponent.K2_SetRelativeTransform` (`self.Scene`) (`KismetMathLibrary.Conv_VectorToTransform` (0.0 0.0 0.0)) false false))
        (:`then_1`
          (`KismetMaterialLibrary.SetVectorParameterValue` "/Game/DissolutionExamples/Materials/MPC_DissolutionMaterialParameterCollection.MPC_DissolutionMaterialParameterCollection" "DissolutionAttractor" (`KismetMathLibrary.Conv_VectorToLinearColor` (`SplineComponent.GetLocationAtDistanceAlongSpline` _trackspline (* (`SplineComponent.GetSplineLength` _trackspline) 0.0) "World"))))
        (:`then_2`
          (`KismetMaterialLibrary.SetVectorParameterValue` "/Game/DissolutionExamples/Materials/MPC_DissolutionMaterialParameterCollection.MPC_DissolutionMaterialParameterCollection" "ForwardVector" (`KismetMathLibrary.MakeColor` 0.0)))
        (:`then_3`
          (for _array_element (`|MakeArray` (`self.BaseColorTexture`) (`self.DepthTexture`) (`self.NormalTexture`))
            (`KismetRenderingLibrary.ClearRenderTarget2D` _array_element))
          (for _array_element_2 _scenecapturecomponents
            (`ActorComponent.K2_DestroyComponent` _array_element_2))
          (`KismetArrayLibrary.Array_Clear` _scenecapturecomponents))))))

(fn `Dissolve`
  (params (Actor :type "Actor Object Reference") (InAsset :type "NiagaraSystem Object Reference"))
  (returns (NiagaraComponents :type "Array of NiagaraComponent Object Reference"))
  (locals (LocalNiagaraSystems :type "NiagaraComponent Object Reference") (LocalNiagaraSystemAssets :type "Array of NiagaraSystem Object Reference"))
  (for _array_element (`self.NiagaraComponents`)
    (`/Engine/EditorBlueprintResources/StandardMacros.IsValid` _array_element
      (:`Is Valid`
        (`KismetArrayLibrary.Array_AddUnique` (`local.LocalNiagaraSystemAssets`) (`NiagaraComponent.GetAsset` _array_element)))))
  (if (== (`KismetArrayLibrary.Array_Find` (`local.LocalNiagaraSystemAssets`) InAsset) -1)
    (bind _returnvalue (`AddComponent|NODE_AddNiagaraComponent-2`))
    (`NiagaraComponent.SetAsset` _returnvalue InAsset)
    (bind _output_get (set `local.LocalNiagaraSystems` _returnvalue))
    (`SceneComponent.K2_AttachToComponent` _output_get (`self.Scene`) "None" "KeepWorld" "KeepWorld" "KeepWorld" true)
    (`|ExecutionSequence`
      (:`then_0`
        (`NiagaraFunctionLibrary.SetTextureObject` _returnvalue "BaseColorTexture" (`self.BaseColorTexture`))
        (`NiagaraFunctionLibrary.SetTextureObject` _returnvalue "NormalTexture" (`self.NormalTexture`))
        (`NiagaraFunctionLibrary.SetTextureObject` _returnvalue "DepthTexture" (`self.DepthTexture`)))
      (:`then_1`
        (`NiagaraComponent.SetVariableVec3` _returnvalue "Center" (`self.K2_GetActorLocation`))
        (`NiagaraComponent.SetNiagaraVariableFloat` _returnvalue "Lifetime" (`self.Lifetime`))
        (`NiagaraComponent.SetNiagaraVariableFloat` _returnvalue "Distance" (`self.MaxDistance`))
        (`NiagaraComponent.SetNiagaraVariableInt` _returnvalue "Width" (`self.Width`))
        (`ActorComponent.Activate` _returnvalue true))
      (:`then_2`
        (return (`|MakeArray` (`local.LocalNiagaraSystems`)))))
    (else
      (return))))

(fn `UserConstructionScript`
  (bind _returnvalue (* (`KismetMathLibrary.Conv_IntToDouble` (`self.Width`)) 0.5))
  (`parent.UserConstructionScript`)
  (`SceneComponent.SetWorldScale3D` (`self.Decal`) (`KismetMathLibrary.MakeVector` _returnvalue _returnvalue (`self.MaxDistance`))))