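; BP_Dissolver sequences Niagara dissolve effects over mapped actors to make them appear or change visibility, labeled with its class name.
; Activate steps through the map with delay-driven manual loops, collecting components from Dissolve, an empty stub here.
; Appearance mode hides all actors first and reveals them after the last effect; otherwise each actor's visibility is set during its step.
; Deactivate breaks the non-appearance loop, destroys the components and unhides all actors.
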(event `/Game/DissolutionExamples/Blueprints/Interface/BP_ActivationInterface.Activate`
  (params (Appearance :type Boolean))
  (bind _duration (`self.Duration`))
  (bind _actorniagarasystemmap (`self.ActorNiagaraSystemMap`))
  (bind _actorsvisibilityduration (`self.ActorsVisibilityDuration`))
  (bind _duration_2 (`self.Duration`))
  (bind _actorniagarasystemmap_2 (`self.ActorNiagaraSystemMap`))
  (if Appearance
    (bind _keys (`BlueprintMapLibrary.Map_Keys` (`self.ActorNiagaraSystemMap`)))
    (for _array_element _keys
      (`self.SetActorHiddenInGame` _array_element true))
    (bind _keys_2 (`BlueprintMapLibrary.Map_Keys` _actorniagarasystemmap_2))
    (bind _arrayelement (`/Game/DissolutionExamples/Blueprints/MacroLibrary/BP_LoopMacroLibrary.OpenForeachLoopWithBreak` _keys_2 :!via `Exec` :!label _label)
      (:`LoopBody`
        (`|ExecutionSequence`
          (:`then_0`
            (bind _niagaracomponents (`self.Dissolve` _arrayelement (`BlueprintMapLibrary.Map_Find` _actorniagarasystemmap_2 _arrayelement)))
            (`KismetArrayLibrary.Array_Append` (`self.NiagaraComponents`) _niagaracomponents))
          (:`then_1`
            (if (> _duration_2 0.0)
              (`KismetSystemLibrary.RetriggerableDelay` _duration_2)
              (goto _label)
              (else
                (goto _label))))))
      (:`Completed`
        (`KismetSystemLibrary.RetriggerableDelay` (`self.AppearanceTime`))
        (bind _keys_3 (`BlueprintMapLibrary.Map_Keys` (`self.ActorNiagaraSystemMap`)))
        (for _array_element_2 _keys_3
          (`self.SetActorHiddenInGame` _array_element_2 false))))
    (else
      (bind _keys_4 (`BlueprintMapLibrary.Map_Keys` _actorniagarasystemmap))
      (bind _arrayelement_2 (`/Game/DissolutionExamples/Blueprints/MacroLibrary/BP_LoopMacroLibrary.OpenForeachLoopWithBreak` _keys_4 :!via `Exec` :!label _label_2)
        (:`LoopBody`
          (`|ExecutionSequence`
            (:`then_0`
              (bind _niagaracomponents_2 (`self.Dissolve` _arrayelement_2 (`BlueprintMapLibrary.Map_Find` _actorniagarasystemmap _arrayelement_2)))
              (`KismetArrayLibrary.Array_Append` (`self.NiagaraComponents`) _niagaracomponents_2))
            (:`then_1`
              (if (> _actorsvisibilityduration 0.0)
                (`KismetSystemLibrary.RetriggerableDelay` _actorsvisibilityduration))
              (`self.SetActorHiddenInGame` _arrayelement_2 (not (`self.ActorsVisibility`)))
              (if (> _duration 0.0)
                (`KismetSystemLibrary.RetriggerableDelay` _duration)
                (goto _label_2)
                (else
                  (goto _label_2))))))))))

(event `/Game/DissolutionExamples/Blueprints/Interface/BP_ActivationInterface.Deactivate`
  (`|ExecutionSequence`
    (:`then_0`
      (goto _label_2 :!via `Break`))
    (:`then_1`
      (for _array_element (`self.NiagaraComponents`)
        (`/Engine/EditorBlueprintResources/StandardMacros.IsValid` _array_element
          (:`Is Valid`
            (`ActorComponent.K2_DestroyComponent` _array_element))))
      (bind _keys (`BlueprintMapLibrary.Map_Keys` (`self.ActorNiagaraSystemMap`)))
      (for _array_element_2 _keys
        (`self.SetActorHiddenInGame` _array_element_2 false))
      (`KismetArrayLibrary.Array_Clear` (`self.NiagaraComponents`)))))

(fn `Dissolve`
  (params (Actor :type "Actor Object Reference") (InAsset :type "NiagaraSystem Object Reference"))
  (returns (NiagaraComponents :type "Array of NiagaraComponent Object Reference"))
  (return))

(fn `UserConstructionScript`
  (`TextRenderComponent.K2_SetText` (`self.TextRender`) (`KismetTextLibrary.Conv_StringToText` (`KismetSystemLibrary.GetClassDisplayName` (`GameplayStatics.GetObjectClass` self)))))