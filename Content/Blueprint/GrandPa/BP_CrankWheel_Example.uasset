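; Example crank wheel actor that rotates a set of linked crank wheels in response to a trigger listener component's continuous percent value.
; Each positive update is compared with the previous one to set the spin direction, and the raw value is printed.
; When IsTest is on, each wheel in the Actor array steps by its own RotateSpeed along this actor's chosen Euler axis, so step size ignores how much the percent changed.
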(event `self.Comp_ListenToTrigger.TriggerConstant`
  (params (Name :type Name) (Distance :type "Float (single-precision)") (Percent :type "Float (single-precision)") (Set :type "/Game/AVRFramework/Structs/Struct_Section Structure") (Velocity :type "Float (single-precision)") (Source :type "Actor Object Reference") (Pawn :type "/Game/AVRFramework/Blueprints/Pawn/BP_Pawn_Base Object Reference"))
  (bind _returnvalue (> Percent 0.0))
  (`KismetSystemLibrary.PrintString` (`KismetStringLibrary.Conv_DoubleToString` Percent) false false)
  (if _returnvalue
    (if (> Percent (`self.OldRotate`))
      (set `self.OldRotate` Percent)
      (set `self.flag` 1.0)
      (else
        (set `self.OldRotate` Percent)
        (set `self.flag` -1.0)))
    (if (and _returnvalue (`self.IsTest`))
      (for _array_element (`self.Actor`)
        (bind _asbp_crank_wheel_example (cast `/Game/Blueprint/GrandPa/BP_CrankWheel_Example` _array_element))
        (`self.AddAngle` (* (`/Game/Blueprint/GrandPa/BP_CrankWheel_Example.RotateSpeed` _asbp_crank_wheel_example) (`self.flag`)) _array_element)))))

(event `AddAngle`
  (params (percent :type "Float (double-precision)") (object :type "Actor Object Reference"))
  (bind (_returnvalue_roll _returnvalue_pitch _returnvalue_yaw) (`KismetMathLibrary.BreakRotator` (`self.K2_GetActorRotation` object)))
  (switch `/Game/Blueprint/Rotate` (`self.RoatateAxis`)
    (:`NewEnumerator0`
      (`self.K2_SetActorRotation` object (`KismetMathLibrary.MakeRotator` (+ _returnvalue_roll percent) _returnvalue_pitch _returnvalue_yaw) false))
    (:`NewEnumerator1`
      (`self.K2_SetActorRotation` object (`KismetMathLibrary.MakeRotator` _returnvalue_roll (+ _returnvalue_pitch percent) _returnvalue_yaw) false))
    (:`NewEnumerator2`
      (`self.K2_SetActorRotation` object (`KismetMathLibrary.MakeRotator` _returnvalue_roll _returnvalue_pitch (+ _returnvalue_yaw percent)) false))))

(fn `UserConstructionScript`)