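; BP_Clock is a clock actor in the GrandPa content that reacts to events from its ListenToTrigger component.
; Constant triggers print their percent and, once it reaches 0.2 while IsAffect is true, enter a DoOnce that drives no further action.
; Single triggers print the section name.
; A Hole.Come call, commented as a dissolve transition, is left unconnected and never runs.
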(event `self.Comp_ListenToTrigger.TriggerConstant`
  (params (Name :type Name) (Distance :type "Float (single-precision)") (Percent :type "Float (single-precision)") (Set :type "/Game/AVRFramework/Structs/Struct_Section Structure") (Velocity :type "Float (single-precision)") (Source :type "Actor Object Reference") (Pawn :type "/Game/AVRFramework/Blueprints/Pawn/BP_Pawn_Base Object Reference"))
  (`KismetSystemLibrary.PrintString` (`KismetStringLibrary.Conv_DoubleToString` Percent))
  (if (and (>= Percent 0.2) (`self.isAffect`))
    (`/Engine/EditorBlueprintResources/StandardMacros.DoOnce` false)))

(event `self.Comp_ListenToTrigger.TriggerSingle`
  (params (Name :type Name) (Section :type "/Game/AVRFramework/Structs/Struct_Section Structure") (Source :type "Actor Object Reference") (Pawn :type "/Game/AVRFramework/Blueprints/Pawn/BP_Pawn_Base Object Reference"))
  (`KismetSystemLibrary.PrintString` (`KismetStringLibrary.Conv_NameToString` Section_Name_2_3833462340DCB130CE3DA7A45D978F38) false false))

(fn `UserConstructionScript`)