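; BP_Door_2 is a door actor Blueprint whose graph only prints debug output.
; It listens to its trigger component's TriggerSingle event and its open component's OpenPercentChanged and activation events.
; All three events feed one PrintString, and the open percent is not passed to it.
; The graph itself contains no door movement logic, and the default BeginPlay, overlap and Tick events are disabled.
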(event `self.Comp_Actor_Trigger.TriggerSingle`
  (params (Name :type Name) (Section :type "/Game/AVRFramework/Structs/Struct_Section Structure") (Source :type "Actor Object Reference") (Pawn :type "/Game/AVRFramework/Blueprints/Pawn/BP_Pawn_Base Object Reference"))
  (`KismetSystemLibrary.PrintString` "Hello" :!label _label))

(event `self.Comp_Actor_Open.OpenPercentChanged`
  (params (Percent :type "Float (single-precision)") (Key :type Name))
  (goto _label))

(event `self.Comp_Actor_Open.OnComponentActivated`
  (params (Component :type "ActorComponent Object Reference") (bReset :type Boolean))
  (goto _label))

(fn `UserConstructionScript`
  (`parent.UserConstructionScript`))